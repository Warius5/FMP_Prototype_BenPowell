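; Battle manager for an auto-battler that runs turn-based fights between the heroes and an enemy.
; Enemy stats come from the clicked map node, then all characters are sorted by Speed into a turn order.
; After the game mode's button event, delayed NextTurn calls cycle through living characters, each damaging a random opponent.
; Death events end the battle, and the menu manager's Next event resets both sides and offers equipment.
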(event Custom|Set%20Up%20Order
  (bind _outactors (Actor|GetAllActorsOfClass "/Game/BenPowell/Characters/BP_BaseCharacter.BP_BaseCharacter_C"))
  (bind _sortedcharacters (CallFunction|SortCharacters _outactors))
  (bind _output_get (Variables|Default|SetTurnOrder _sortedcharacters))
  (bind _output_get_2 (Variables|Default|SetTurnOver (Utilities|Array|Length _output_get)))
  (Development|PrintString (Utilities|String|ToString(Integer) _output_get_2)))

(event Custom|Combat
  (Development|PrintString "Combat")
  (Variables|Default|SetcurrentTurnActor (Utilities|Array|Get(acopy) (Variables|Default|GetTurnOrder) (Variables|Default|GetturnIndex)))
  (CallFunction|AttackLogic))

(event Custom|Next%20Turn
  (if (Variables|Default|GetBattleComplete)
    (CallFunction|Reset)
    (else
      (Development|PrintString (Utilities|String|ToString(Boolean) (Variables|Default|GetTurning?)))
      (if (not (Variables|Default|GetTurning?))
        (Variables|Default|SetTurning? true)
        (Development|PrintString "Begin")
        (if (< (Variables|Default|GetturnIndex) (Variables|Default|GetTurnOver))
          (bind _alive (|CheckCurentAlive))
          (if _alive
            (CallFunction|Combat)
            (goto _label execute2)
            (else
              (|CollapseGraph_2 :!label _label)
              (CallFunction|NextTurn)))
          (else
            (CallFunction|Reset)
            (Utilities|FlowControl|Delay 1.0)
            (Variables|Default|SetTurning? false)
            (CallFunction|NextTurn)))))))

(event Custom|Reset
  (bind _turnorder (Variables|Default|GetTurnOrder))
  (for _array_element _turnorder
    (Default|AttackDone _array_element)
    (Variables|Default|SetturnIndex 0)
    (Variables|Default|SetTurnOver (Utilities|Array|Length _turnorder))))

(event Custom|Delay
  (params (Current :type BP%20Base%20Character%20Object%20Reference))
  (Development|PrintString "Delay STARt")
  (Utilities|FlowControl|Delay 3e+01)
  (Default|AttackDone Current))

(event Custom|Start%20Combat
  (Viewport|RemoveAllWidgets)
  (CallFunction|NextTurn))

(event Custom|Dead
  (params (Character :type BP%20Base%20Character%20Object%20Reference))
  (bind _output_get (Variables|Default|SetCharacter Character))
  (if (Variables|/Game/BenPowell/Characters/BP_BaseCharacter.BP_BaseCharacter_C|GetEnemy _output_get)
    (Variables|Default|SetBattleComplete true :!label _label)
    (Development|PrintString "GAME OVER")
    (Default|CallGameOverDispatch (Variables|Default|GetCharacter))
    (else
      (Variables|Default|SetAliveHeroes (- (Variables|Default|GetAliveHeroes) 1))
      (Variables|/Script/Engine.Actor|SetTags (Variables|Default|GetCharacter) (Variables|Default|Getempty%28dead))
      (if (not (> (Variables|Default|GetAliveHeroes) 0))
        (Development|PrintString "Everyone Is Dead")
        (goto _label)))))

(event Custom|Next_Event
  (params (NewParam :type BP%20Base%20Character%20Object%20Reference))
  ;[1 1 1] Resetting
  (|CollapseGraph_1 NewParam)
  (CallFunction|EnemySetUp NewParam)
  (CallFunction|HeroSetUp)
  (bind _asbp_auto_bgame_mode (Utilities|Casting|CastToBP_AutoBGameMode (Game|GetGameMode)))
  (Variables|/Game/BenPowell/BP_AutoBGameMode.BP_AutoBGameMode_C|SetItemsToGive _asbp_auto_bgame_mode 3)
  (Default|CallChangeEquip _asbp_auto_bgame_mode)
  (Development|PrintString "Hello"))

(event Custom|Hero%20Set%20up
  ;[1 1 1] Enemy Set UP
  (bind _outactors (Actor|GetAllActorsOfClass "/Game/BenPowell/Characters/BPC_Hero.BPC_Hero_C"))
  (for _array_element _outactors
    (bind _array_element_2 (|SettingHealths _array_element))
    (Default|SetText _array_element_2)
    (Variables|/Script/Engine.Actor|SetTags (Variables|Default|GetArray%20Element) (Variables|Default|GetAliveTags)))
  (Variables|Default|SetAliveHeroes 3))

(event EventBeginPlay
  (bind _outactors (Actor|GetAllActorsOfClass "/Game/BenPowell/Characters/BPC_Enemy.BPC_Enemy_C"))
  (bind _asbpc_enemy (Utilities|Casting|CastToBPC_Enemy (.ReturnValue (Actor|FindNearestActor "0, 0, 0" _outactors))))
  (Variables|Default|SetEnemyVar _asbpc_enemy)
  (CallFunction|EnemySetUp (Variables|Default|GetEnemyVar))
  (bind _outactors_2 (Actor|GetAllActorsOfClass "/Game/BenPowell/BP_MenuManager.BP_MenuManager_C"))
  (Variables|Default|SetMenuManager (.ReturnValue (Actor|FindNearestActor "0, 0, 0" _outactors_2)))
  (bind _asbp_auto_bgame_mode (Utilities|Casting|CastToBP_AutoBGameMode (Game|GetGameMode)))
  (EventDispatchers|BindEventtoPressButton _asbp_auto_bgame_mode (delegate Custom|Start%20Combat))
  (EventDispatchers|BindEventtoNextTurn (Variables|Default|GetAs%20BP%20Main%20View) (EventDispatchers|CreateEvent :!event Custom|Next%20Turn))
  (bind _outactors_3 (Actor|GetAllActorsOfClass "/Game/BenPowell/Characters/BP_BaseCharacter.BP_BaseCharacter_C"))
  (for _array_element _outactors_3
    (EventDispatchers|BindEventtoDead _array_element (delegate Custom|Dead))
    (bind _asbp_menu_manager (Utilities|Casting|CastToBP_MenuManager (Variables|Default|GetMenuManager)))
    (EventDispatchers|BindEventtoNext _asbp_menu_manager (delegate Custom|Next_Event))
    (Development|PrintString "set up")
    (CallFunction|EnemySetUp (Variables|Default|GetEnemyVar))))

(event Collision|EventActorBeginOverlap
  (params (OtherActor :type Actor%20Object%20Reference)))

(fn ConstructionScript)

(fn SortCharacters
  (params (CharactersToSort :type Array%20of%20BP%20Base%20Character%20Object%20References))
  (Variables|Default|SetSorted CharactersToSort)
  (for _index (range 0 (- (Utilities|Array|Length (Variables|Default|GetSorted)) 2))
    (for _index_2 (range (+ _index 1) (- (Utilities|Array|Length (Variables|Default|GetSorted)) 1))
      (bind _a_bigger (CallFunction|ActorSortFunction (Utilities|Array|Get(acopy) (Variables|Default|GetSorted) _index_2) (Utilities|Array|Get(acopy) (Variables|Default|GetSorted) _index)))
      (if _a_bigger
        (Utilities|Array|Swap (Variables|Default|GetSorted) _index _index_2))))
  (return (Variables|Default|GetSorted)))

(fn ActorSortFunction
  (params (ActorA :type BP%20Base%20Character%20Object%20Reference) (ActorB :type BP%20Base%20Character%20Object%20Reference))
  (return (> (Variables|/Game/BenPowell/Characters/BP_BaseCharacter.BP_BaseCharacter_C|GetSpeed ActorA) (Variables|/Game/BenPowell/Characters/BP_BaseCharacter.BP_BaseCharacter_C|GetSpeed ActorB))))

(fn DamageCalc
  (params (ToFindClass :type Array%20of%20BP%20Base%20Character%20Object%20References))
  (bind _output_get (Variables|Default|SetTheTarget (.OutItem (Utilities|Array|Random ToFindClass))))
  (Variables|/Game/BenPowell/Characters/BP_BaseCharacter.BP_BaseCharacter_C|SetHealth _output_get (- (Variables|/Game/BenPowell/Characters/BP_BaseCharacter.BP_BaseCharacter_C|GetHealth _output_get) (Variables|/Game/BenPowell/Characters/BP_BaseCharacter.BP_BaseCharacter_C|GetDamage (Variables|Default|GetcurrentTurnActor))))
  (Default|SetText _output_get))

(fn AttackLogic
  (params (CurrentTurnActor :type BP%20Base%20Character%20Object%20Reference))
  (bind _currentturnactor (Variables|Default|GetcurrentTurnActor))
  (Development|PrintString "Attack Logic")
  (Default|ShowAttack _currentturnactor)
  (if (Variables|/Game/BenPowell/Characters/BP_BaseCharacter.BP_BaseCharacter_C|GetEnemy _currentturnactor)
    (bind _outactors (Actor|GetAllActorsOfClasswithTag "/Game/BenPowell/Characters/BPC_Hero.BPC_Hero_C" "Alive"))
    (if (Utilities|Array|IsEmpty _outactors)
      (return)
      (else
        (CallFunction|DamageCalc _outactors)))
    (else
      (bind _outactors_2 (Actor|GetAllActorsOfClass "/Game/BenPowell/Characters/BPC_Enemy.BPC_Enemy_C"))
      (CallFunction|DamageCalc _outactors_2))))

(event Custom|Enemy%20Set%20Up
  (params (Enemy :type BP%20Base%20Character%20Object%20Reference))
  (bind _asbp_node (Utilities|Casting|CastToBP_Node (Variables|/Game/BenPowell/MapSide/BP_Map.BP_Map_C|GetCurrentlyClicked (Variables|Default|GetMap_Reference))))
  (Variables|Default|SetEnemy Enemy)
  (Variables|/Game/BenPowell/Characters/BP_BaseCharacter.BP_BaseCharacter_C|SetHealth (Variables|Default|GetEnemy) (.health (Variables|/Game/BenPowell/MapSide/BP_Node.BP_Node_C|GetEnemyStats _asbp_node)))
  (Variables|/Game/BenPowell/Characters/BP_BaseCharacter.BP_BaseCharacter_C|SetSpeed (Variables|Default|GetEnemy) (.speed (Variables|/Game/BenPowell/MapSide/BP_Node.BP_Node_C|GetEnemyStats _asbp_node)))
  (Variables|/Game/BenPowell/Characters/BP_BaseCharacter.BP_BaseCharacter_C|SetDamage (Variables|Default|GetEnemy) (.damage (Variables|/Game/BenPowell/MapSide/BP_Node.BP_Node_C|GetEnemyStats _asbp_node)))
  (Default|SetText (Variables|Default|GetEnemy))
  (Default|SetTextDamage (Variables|Default|GetEnemy))
  (CallFunction|SetUpOrder))