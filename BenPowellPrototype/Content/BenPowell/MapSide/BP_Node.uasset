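; BP_Node is a clickable node on a branching map, holding left and right child links and rolled enemy stats.
; SelectDifficulty picks its own or ParentNode's depth at random, or the boss tier, then rolls health, damage and speed within that tier's ranges.
; Clicks only count on children of BP_Map's current node, notifying BPI_NodeInterface actors.
; Macros recolor borders to show selected and reachable nodes on BeginPlay and valid clicks.
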(event Custom|SelectDifficulty
  ;[1 1 1] Checks if its a boss or normal node, if its not, it gets the difficulty by using a random bool to pick between two options, the current depth or the previous depth. This then translates into the switch and uses a function library to set the enemy events stats. This is then fed into the structpop function.
  (if (not (Variables|Default|GetIsBoss))
    (Variables|Default|SetDifficultyChoose (Math|Integer|SelectInt (Variables|BP_Node_C|GetDepth (Variables|Default|GetParentNode)) (Variables|Default|GetDepth) (Math|Random|RandomBool)))
    (else
      (Variables|Default|SetDifficultyChoose 6)))
  (switch int (Variables|Default|GetDifficultyChoose)
    (:Default
      (bind _stats (CallFunction|RootGet :!label _label))
      (Variables|Default|SetEnemyEvent _stats))
    (:1
      (goto _label))
    (:2
      (bind _stats_2 (CallFunction|1Get))
      (Variables|Default|SetEnemyEvent _stats_2))
    (:3
      (bind _stats_3 (CallFunction|2Get))
      (Variables|Default|SetEnemyEvent _stats_3))
    (:4
      (bind _stats_4 (CallFunction|3Get))
      (Variables|Default|SetEnemyEvent _stats_4))
    (:5
      (bind _stats_5 (CallFunction|4Get))
      (Variables|Default|SetEnemyEvent _stats_5))
    (:6
      (bind _stats_6 (CallFunction|BossGet))
      (Variables|Default|SetEnemyEvent _stats_6)))
  (bind _newparam (CallFunction|Structpop (Variables|Default|GetEnemyEvent)))
  (Variables|Default|SetEnemyStats _newparam))

(event EventBeginPlay
  (|ChangingtheMAterials_2_2))

(event Collision|EventActorBeginOverlap
  (params (OtherActor :type Actor%20Object%20Reference)))

(event EventTick
  (params (DeltaSeconds :type Float%20%28single-precision%29)))

(event MouseInput|EventActorOnClicked
  (params (ButtonPressed :type Key%20Structure :default "None"))
  ;[1 1 1] When a node is clicked on the map, it checks whether that node is a valid node and if not does not continue. If it does, it changes the materials of the new node and left and right nodes. Then triggers an interface, which would be on the BP_map.
  (bind _outactors (Actor|GetAllActorswithInterface "/Game/BenPowell/MapSide/BPI_NodeInterface.BPI_NodeInterface_C"))
  (bind _asbp_map (Utilities|Casting|CastToBP_Map (Utilities|Array|Get(acopy) _outactors)))
  (bind _asbp_node (Utilities|Casting|CastToBP_Node (Variables|/Game/BenPowell/MapSide/BP_Map.BP_Map_C|GetCurrentlyClicked _asbp_map)))
  (if (or (== (Variables|BP_Node_C|GetLeftNode _asbp_node) self) (== (Variables|BP_Node_C|GetRightNode _asbp_node) self))
    (|ChangingtheMAterials
      (:then
        _)
      (:Is%20Not%20Valid
        _))
    (bind _outactors_2 (Actor|GetAllActorswithInterface "/Game/BenPowell/MapSide/BPI_NodeInterface.BPI_NodeInterface_C"))
    (for _array_element _outactors_2
      (Class|BPINodeInterface|NodeSelected(Message) _array_element (Variables|Default|GetLocationAbove) self))
    (else
      (Development|PrintString "not valid"))))

(fn ConstructionScript
  (Variables|Default|SetParentNode self)
  (Rendering|Material|SetMaterial (Variables|Default|GetBorder) 0 "/Game/BenPowell/MapSide/Materials/M_Non.M_Non")
  (Variables|Default|SetLocationAbove (Transformation|GetWorldLocation (Variables|Default|GetMovePoint))))

(fn NodeSelected
  (params (Positions :type Vector :default "0, 0, 0") (NewParam :type Boolean) (selectedNode :type Boolean) (NewParamsdg1 :type BP%20Node%20Object%20Reference))
  (return))

(fn Structpop
  (params (inputStruct :type S%20Eneny%20Event%20Structure))
  ;[1 1 1] Gets a random number from the ranges
  (return (Utilities|Struct|MakeS_EnemyStats (Math|Random|RandomIntegerinRange (.healthlow inputStruct) (.healthup inputStruct)) (Math|Random|RandomIntegerinRange (.damagelow inputStruct) (.damageup inputStruct)) (Math|Random|RandomIntegerinRange (.speedlow inputStruct) (.speedup inputStruct)) (.difficulty inputStruct))))