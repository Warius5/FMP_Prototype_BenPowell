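; Item manager for an auto-battler that applies equipment bonuses to the selected hero.
; On BeginPlay it binds to player controller and game mode dispatchers for hero selection and Big Armour or Big Sword presses.
; Each press, if a hero is selected and items remain, adds the DT_Items bonus to health or damage, updating max stats and text.
; It then re-enables selecting, decrements the item count and notifies the game mode.
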(event Custom|ClearSelected
  (Variables|Default|SetSected%20Hero 0))

(event Custom|PressBigArmour_Event
  (params (BigArmour :type Base%20Inventory%20Item%20Object%20Reference))
  (bind _sected_hero (Variables|Default|GetSected%20Hero))
  ;[1 1 1] Gets the the data table row for the bigarmour and uses that as the value to change the health of the selected character
  (if (Utilities|IsValid (Variables|Default|GetSected%20Hero))
    (if (> (Variables|/Game/BenPowell/BP_AutoBGameMode.BP_AutoBGameMode_C|GetItemsToGive (Variables|Default|GetAs%20BP%20Auto%20BGame%20Mode)) 0)
      (bind _returnvalue (Utilities|GetDataTableRow "/Game/BenPowell/Characters/Items/DT_Items.DT_Items" "BigArmour")
        (:then
          (bind _output_get (Variables|/Game/BenPowell/Characters/BP_BaseCharacter.BP_BaseCharacter_C|SetHealth _sected_hero (+ (.AddHealth (Utilities|Struct|BreakS_Item _returnvalue)) (Variables|/Game/BenPowell/Characters/BP_BaseCharacter.BP_BaseCharacter_C|GetHealth _sected_hero))))
          (Variables|/Game/BenPowell/Characters/BPC_Hero.BPC_Hero_C|SetMax%20Stats _sected_hero (Utilities|Struct|MakeS_EnemyStats _output_get (.damage (Variables|/Game/BenPowell/Characters/BPC_Hero.BPC_Hero_C|GetMax%20Stats _sected_hero)) (.speed (Variables|/Game/BenPowell/Characters/BPC_Hero.BPC_Hero_C|GetMax%20Stats _sected_hero)) 0))
          (Default|SetText _sected_hero)
          (Variables|/Game/BenPowell/BP_AutoBGamePlayerController.BP_AutoBGamePlayerController_C|SetSelecting (Variables|Default|GetAs%20BP%20Auto%20BGame%20Player%20Controller) true)
          (Variables|/Game/BenPowell/BP_AutoBGameMode.BP_AutoBGameMode_C|SetItemsToGive (Variables|Default|GetAs%20BP%20Auto%20BGame%20Mode) (- (Variables|/Game/BenPowell/BP_AutoBGameMode.BP_AutoBGameMode_C|GetItemsToGive (Variables|Default|GetAs%20BP%20Auto%20BGame%20Mode)) 1))
          (Default|CallChangeEquip (Variables|Default|GetAs%20BP%20Auto%20BGame%20Mode)))))))

(event Custom|PressBigSword_Event
  (params (BigSword :type Base%20Inventory%20Item%20Object%20Reference))
  (bind _sected_hero (Variables|Default|GetSected%20Hero))
  (bind _sected_hero_2 (Variables|Default|GetSected%20Hero))
  (bind _as_bp_auto_bgame_mode (Variables|Default|GetAs%20BP%20Auto%20BGame%20Mode))
  ;[1 1 1] Gets the the data table row for the bigsword and uses that as the value to change the damage of the selected character
  (if (Utilities|IsValid (Variables|Default|GetSected%20Hero))
    (if (> (Variables|/Game/BenPowell/BP_AutoBGameMode.BP_AutoBGameMode_C|GetItemsToGive (Variables|Default|GetAs%20BP%20Auto%20BGame%20Mode)) 0)
      (bind _returnvalue (Utilities|GetDataTableRow "/Game/BenPowell/Characters/Items/DT_Items.DT_Items" "BigSword")
        (:then
          (bind _output_get (Variables|/Game/BenPowell/Characters/BP_BaseCharacter.BP_BaseCharacter_C|SetDamage _sected_hero (+ (.AddDamage (Utilities|Struct|BreakS_Item _returnvalue)) (Variables|/Game/BenPowell/Characters/BP_BaseCharacter.BP_BaseCharacter_C|GetDamage _sected_hero))))
          (Variables|/Game/BenPowell/Characters/BPC_Hero.BPC_Hero_C|SetMax%20Stats _sected_hero_2 (Utilities|Struct|MakeS_EnemyStats (.health (Variables|/Game/BenPowell/Characters/BPC_Hero.BPC_Hero_C|GetMax%20Stats _sected_hero_2)) _output_get (.speed (Variables|/Game/BenPowell/Characters/BPC_Hero.BPC_Hero_C|GetMax%20Stats _sected_hero_2)) 0))
          (Default|SetTextDamage (Variables|Default|GetSected%20Hero))
          (Variables|/Game/BenPowell/BP_AutoBGamePlayerController.BP_AutoBGamePlayerController_C|SetSelecting (Variables|Default|GetAs%20BP%20Auto%20BGame%20Player%20Controller) true)
          (Variables|/Game/BenPowell/BP_AutoBGameMode.BP_AutoBGameMode_C|SetItemsToGive _as_bp_auto_bgame_mode (- (Variables|/Game/BenPowell/BP_AutoBGameMode.BP_AutoBGameMode_C|GetItemsToGive _as_bp_auto_bgame_mode) 1))
          (Default|CallChangeEquip _as_bp_auto_bgame_mode))))))

(event Custom|SendHero_Event
  (params (Selecting :type Boolean) (SelectHero :type BPC%20Hero%20Object%20Reference))
  (Variables|Default|SetSelecting Selecting)
  (Variables|Default|SetSected%20Hero SelectHero))

(event EventBeginPlay
  ;[1 1 1] Sets up theevent binds that will be triggered from equop buttons or selecting a Hero
  (bind _asbp_auto_bgame_mode (Utilities|Casting|CastToBP_AutoBGameMode (Game|GetGameMode)))
  (Variables|Default|SetAs%20BP%20Auto%20BGame%20Mode _asbp_auto_bgame_mode)
  (bind _asbp_auto_bgame_player_controller (Utilities|Casting|CastToBP_AutoBGamePlayerController (Game|GetPlayerController 0)))
  (bind _output_get (Variables|Default|SetAs%20BP%20Auto%20BGame%20Player%20Controller _asbp_auto_bgame_player_controller))
  (EventDispatchers|BindEventtoSendHero _output_get (EventDispatchers|CreateEvent :!event Custom|SendHero_Event))
  (EventDispatchers|BindEventtoPressBigArmour (Variables|Default|GetAs%20BP%20Auto%20BGame%20Mode) (EventDispatchers|CreateEvent :!event Custom|PressBigArmour_Event))
  (EventDispatchers|BindEventtoPressBigSword (Variables|Default|GetAs%20BP%20Auto%20BGame%20Mode) (EventDispatchers|CreateEvent :!event Custom|PressBigSword_Event)))

(event Collision|EventActorBeginOverlap
  (params (OtherActor :type Actor%20Object%20Reference)))

(event EventTick
  (params (DeltaSeconds :type Float%20%28single-precision%29)))

(fn ConstructionScript)