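; Player controller for the auto-battler that lets the player click a hero during the equip phase and broadcasts the choice.
; Big sword and big armour press events arm selection, though their game mode bindings here are disconnected.
; While the game mode's OnEquip is set, a left click line-traces from the cursor, stores the hit BPC_Hero, clears selection and calls SendHero.
; Inventory-add logic is also unconnected.
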(event Custom|PressBigArmour_Event
  (params (BigArmour :type Base%20Inventory%20Item%20Object%20Reference))
  (Development|PrintString "gamemode EVent")
  (Variables|Default|SetSelecting true))

(event Custom|PressBigSword_Event
  (params (BigSword :type Base%20Inventory%20Item%20Object%20Reference))
  (Development|PrintString "gamemode EVent")
  (Variables|Default|SetSelecting true))

(event EventBeginPlay)

(event EventTick
  (params (DeltaSeconds :type Float%20%28single-precision%29)))

(event Input|ActionEvents|InputActionLeftClick
  (params (Key :type Key%20Structure :default "None"))
  (bind _returnvalue (Game|GetPlayerController 0))
  (bind _self self)
  (bind (_locationx _locationy) (Game|Player|GetMousePosition _returnvalue))
  (bind (_worldposition _worlddirection) (Class|GameplayStatics|DeprojectScreentoWorld _self (Math|Vector2D|MakeVector2D _locationx _locationy)))
  (:Pressed
    (bind _asbp_auto_bgame_mode (Utilities|Casting|CastToBP_AutoBGameMode (Game|GetGameMode)))
    (if (Variables|/Game/BenPowell/BP_AutoBGameMode.BP_AutoBGameMode_C|GetOnEquip _asbp_auto_bgame_mode)
      (if (Variables|Default|GetSelecting)
        (bind _outhit (Collision|LineTraceByChannel _worldposition (+ _worldposition (* _worlddirection 1e+03)) "TraceTypeQuery1" false 0 "Persistent"))
        (Development|PrintString (Utilities|GetDisplayName (.HitActor (Collision|BreakHitResult _outhit))))
        (bind _asbpc_hero (Utilities|Casting|CastToBPC_Hero (.HitActor (Collision|BreakHitResult _outhit))))
        (if (Utilities|IsValid _asbpc_hero)
          (bind _output_get (Variables|Default|SetSectedHero _asbpc_hero))
          (Development|PrintString (Utilities|GetDisplayName _output_get))
          (Development|PrintString "Selected")
          (bind _output_get_2 (Variables|Default|SetSelecting false))
          (Default|CallSendHero _output_get_2 _output_get))))))

(fn ConstructionScript)