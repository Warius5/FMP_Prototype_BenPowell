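; BP_MenuManager is the actor that switches the auto-battler's UI between opening, start, equip and game-over screens.
; On BeginPlay it shows the opening widget and binds to game mode dispatchers for start, equip and back, which swap widgets and toggle the OnEquip flag.
; It also binds to the battle manager's game-over dispatcher, showing the result screen and, when an enemy died, triggering back and CallNext after a delay.
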(event Custom|OpeningStart_Event
  (Viewport|RemoveAllWidgets)
  (bind _returnvalue (UserInterface|CreateWidget "/Game/BenPowell/UI/StartMenu.StartMenu_C"))
  (bind _output_get (Variables|Default|SetButton%20Screen _returnvalue))
  (UserInterface|Viewport|AddtoViewport _output_get 0))

(event Custom|EquipButton_Event
  (bind _asbp_auto_bgame_mode (Utilities|Casting|CastToBP_AutoBGameMode (Game|GetGameMode)))
  (Variables|/Game/BenPowell/BP_AutoBGameMode.BP_AutoBGameMode_C|SetOnEquip _asbp_auto_bgame_mode true)
  (Viewport|RemoveAllWidgets)
  (bind _returnvalue (UserInterface|CreateWidget "/Game/BenPowell/UI/EquipMenu.EquipMenu_C"))
  (UserInterface|Viewport|AddtoViewport _returnvalue 0))

(event Custom|GameOverDispatch_Event
  (params (Character :type BP%20Base%20Character%20Object%20Reference))
  (bind _enemy (Variables|/Game/BenPowell/Characters/BP_BaseCharacter.BP_BaseCharacter_C|GetEnemy Character))
  (Development|PrintString "death")
  (bind _returnvalue (UserInterface|CreateWidget "/Game/BenPowell/UI/GamerOver.GamerOver_C"))
  (UserInterface|Viewport|AddtoViewport _returnvalue 0)
  (Development|PrintString "widget")
  (bind _output_get (Variables|Default|SetGame%20Over%20Screen _returnvalue))
  (Default|Visibleee _output_get _enemy)
  (UserInterface|Viewport|AddtoViewport _output_get 0)
  (if _enemy
    (Utilities|FlowControl|Delay 3.0)
    (CallFunction|BackButtonEvent)
    (Default|CallNext Character)))

(event Custom|BackButton_Event
  (bind _asbp_auto_bgame_mode (Utilities|Casting|CastToBP_AutoBGameMode (Game|GetGameMode)))
  (Variables|/Game/BenPowell/BP_AutoBGameMode.BP_AutoBGameMode_C|SetOnEquip _asbp_auto_bgame_mode false)
  (Viewport|RemoveAllWidgets)
  (bind _returnvalue (UserInterface|CreateWidget "/Game/BenPowell/UI/StartMenu.StartMenu_C"))
  (bind _output_get (Variables|Default|SetButton%20Screen _returnvalue))
  (UserInterface|Viewport|AddtoViewport _output_get 0))

(event EventBeginPlay
  (bind _asbp_auto_bgame_mode (Utilities|Casting|CastToBP_AutoBGameMode (Game|GetGameMode)))
  (EventDispatchers|BindEventtoOpeningStart _asbp_auto_bgame_mode (delegate Custom|OpeningStart_Event))
  (EventDispatchers|BindEventtoEquipButton _asbp_auto_bgame_mode (delegate Custom|EquipButton_Event))
  (EventDispatchers|BindEventtoBackButton _asbp_auto_bgame_mode (delegate Custom|BackButton_Event))
  (bind _returnvalue (UserInterface|CreateWidget "/Game/BenPowell/UI/Opening.Opening_C"))
  (UserInterface|Viewport|AddtoViewport _returnvalue 0)
  (bind _outactors (Actor|GetAllActorsOfClass "/Game/BenPowell/BP_BattleManager.BP_BattleManager_C"))
  (bind _output_get (Variables|Default|SetBattleManager (.ReturnValue (Actor|FindNearestActor "0, 0, 0" _outactors))))
  (bind _asbp_battle_manager (Utilities|Casting|CastToBP_BattleManager _output_get))
  (EventDispatchers|BindEventtoGameOverDispatch _asbp_battle_manager (delegate Custom|GameOverDispatch_Event)))

(event Collision|EventActorBeginOverlap
  (params (OtherActor :type Actor%20Object%20Reference)))

(event EventTick
  (params (DeltaSeconds :type Float%20%28single-precision%29)))

(fn ConstructionScript)