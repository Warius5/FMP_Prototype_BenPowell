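; BP_MainView is an actor Blueprint that handles player input and screen UI for a turn-based combat game.
; On BeginPlay it adds a GamerOver widget to the viewport, and pressing Next Action calls NextTurn.
; An older initiative system, which sorts BP_BaseCharacter actors by Speed and loops their attacks, remains only as disconnected nodes.
; Its SortOrder, StartTurns and AttackTurn events are empty.
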(event Custom|Position%20Found%20Break
  (bind _initiativearray (Variables|Default|GetInitiativeArray))
  (bind _returnvalue (Utilities|Array|LastIndex _initiativearray))
  (Utilities|Array|ForEachLoopwithBreak (Variables|Default|GetInitiativeArray)) ; enters at Break
)

(event Custom|StartTurns)

(event Custom|AttackTurn)

(event Custom|SortOrder)

(event Collision|EventActorBeginOverlap
  (params (OtherActor :type Actor%20Object%20Reference)))

(event EventBeginPlay
  (bind _returnvalue (UserInterface|CreateWidget "/Game/BenPowell/UI/GamerOver.GamerOver_C"))
  (bind _output_get (Variables|Default|SetGameOverScreen _returnvalue))
  (UserInterface|Viewport|AddtoViewport _output_get 0))

(event Input|ActionEvents|InputActionNextAction
  (params (Key :type Key%20Structure :default "None"))
  (:Pressed
    (Default|CallNextTurn)))

(event Input|KeyboardEvents|X
  (params (Key :type Key%20Structure :default "None")))

(event Input|KeyboardEvents|C
  (params (Key :type Key%20Structure :default "None"))
  ;[1 1 1] Comment
)

(fn ConstructionScript)