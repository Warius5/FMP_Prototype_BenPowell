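; BP_AudioManager is an actor Blueprint that plays background music continuously, alternating between two medieval tracks.
; On BeginPlay it starts its CurrentAudio component and binds that component's OnAudioFinished event to PlayNextTrack.
; PlayNextTrack sets the goofy or hip track based on TrackIndex, plays it, then flips the index, so each finished track triggers the next without Tick.
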(event Custom|PlayNextTrack
  ;[1 1 1] Alternates music being played using track index
  (if (== (Variables|Default|GetTrackIndex) 0)
    (Audio|Components|Audio|SetSound (Variables|Default|GetCurrentAudio) "/Game/BenPowell/Music/GoofyMedievalMusic.GoofyMedievalMusic")
    (else
      (Audio|Components|Audio|SetSound (Variables|Default|GetCurrentAudio) "/Game/BenPowell/Music/HipMedievalMusic.HipMedievalMusic")))
  (Audio|Components|Audio|Play (Variables|Default|GetCurrentAudio) 0.0)
  (Variables|Default|SetTrackIndex (Math|Integer|%(Integer) (+ (Variables|Default|GetTrackIndex) 1) 2)))

(event EventBeginPlay
  ;[1 1 1] Starts the music and binds the ending audio to the PlayNextTrack event
  (Audio|Components|Audio|Play (Variables|Default|GetCurrentAudio) 0.0)
  (EventDispatchers|BindEventtoOnAudioFinished (Variables|Default|GetCurrentAudio) (delegate Custom|PlayNextTrack)))

(event Collision|EventActorBeginOverlap
  (params (OtherActor :type Actor%20Object%20Reference)))

(event EventTick
  (params (DeltaSeconds :type Float%20%28single-precision%29)))

(fn ConstructionScript)